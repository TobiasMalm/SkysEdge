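; Elevator Blueprint that moves its Elevator component up or down when something overlaps its trigger box.
; Each overlap while idle flips HasGoneUp and replays the Move timeline, with IsMoving blocking retriggers until it finishes.
; Every timeline update adds the Pos value as an unswept relative offset, negated for descent, so movement accumulates per tick rather than interpolating between fixed endpoints.
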(event OnComponentBeginOverlap(TriggerBox)
  (params (OtherActor :type Actor%20Object%20Reference) (OtherComp :type Primitive%20Component%20Object%20Reference) (OtherBodyIndex :type Integer))
  (bind _elevator (Variables|Default|GetElevator))
  (if (not (Variables|Default|GetIsMoving))
    (Variables|Default|SetIsMoving true)
    (if (Variables|Default|GetHasGoneUp)
      (Variables|Default|SetHasGoneUp false)
      (bind _pos (Timeline|Move PlayFromStart)
        (:Update
          (if (Variables|Default|GetHasGoneUp)
            (Transformation|AddRelativeLocation _elevator _pos false)
            (else
              (Transformation|AddRelativeLocation _elevator (* _pos -1.0) false))))
        (:Finished
          (Variables|Default|SetIsMoving false)))
      (else
        (Variables|Default|SetHasGoneUp true)
        (Timeline|Move PlayFromStart)))))

(fn ConstructionScript)