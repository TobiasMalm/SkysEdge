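; A flickering light that buzzes as something approaches and blows out when it gets closer.
; BeginPlay loops random brightness until OuterTrigger's overlap flag is seen, then holds it bright and ends the loop; entering OuterTrigger also starts BuzzingSound.
; InnerTrigger fires once: a few rapid flickers, an intense flash, then the light hides, a bang plays, buzzing stops and Sparks activate briefly.
; The construction script moves BuzzingSound to the light's location.
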(event OnComponentBeginOverlap(InnerTrigger)
  (params (OtherActor :type Actor%20Object%20Reference) (OtherComp :type Primitive%20Component%20Object%20Reference) (OtherBodyIndex :type Integer))
  (bind _sparks (Variables|Default|GetSparks))
  (bind _pointlight1 (Variables|Default|GetPointLight1))
  (if (not (Variables|Default|GetisExploded))
    (Variables|Default|SetisExploded true)
    (Class|LightComponent|SetBrightness (Variables|Default|GetPointLight1) (Math|Random|RandomFloatinRange 0.0 1e+04) :!label _label)
    (Utilities|FlowControl|Delay 0.05)
    (if (< (Variables|Default|GetI) (Math|Random|RandomIntegerinRange 2 4))
      (Variables|Default|SetI (+ (Variables|Default|GetI) 1))
      (goto _label)
      (else
        (Class|LightComponent|SetBrightness (Variables|Default|GetPointLight1) 2e+06)
        (Utilities|FlowControl|Delay 0.1)
        (Rendering|SetVisibility _pointlight1 false false)
        (Audio|PlaySoundatLocation "/Game/Audio/Template1rst_WeaponFire02.Template1rst_WeaponFire02" (Transformation|GetWorldLocation _pointlight1))
        (Audio|Components|Audio|Stop (Variables|Default|GetBuzzingSound))
        (Rendering|ToggleVisibility _sparks false)
        (Components|Activation|SetActive _sparks true true)
        (Utilities|FlowControl|Delay 0.5)
        (Rendering|ToggleVisibility _sparks false)
        (Components|Activation|SetActive _sparks false false)))))

(event OnComponentBeginOverlap(OuterTrigger)
  (params (OtherActor :type Actor%20Object%20Reference) (OtherComp :type Primitive%20Component%20Object%20Reference) (OtherBodyIndex :type Integer))
  (Variables|Default|SetIsOverlapping true)
  (Audio|Components|Audio|Play (Variables|Default|GetBuzzingSound) 0.0))

(event OnComponentEndOverlap(OuterTrigger)
  (params (OtherActor :type Actor%20Object%20Reference) (OtherComp :type Primitive%20Component%20Object%20Reference) (OtherBodyIndex :type Integer))
  (Variables|Default|SetIsOverlapping false))

(event EventBeginPlay
  (bind _pointlight1 (Variables|Default|GetPointLight1))
  (if (Variables|Default|GetIsOverlapping) :!label _label
    (Class|LightComponent|SetBrightness _pointlight1 1e+04)
    (else
      (Class|LightComponent|SetBrightness _pointlight1 (Math|Random|RandomFloatinRange 0.0 5e+03))
      (Utilities|FlowControl|Delay 0.1)
      (goto _label))))

(fn ConstructionScript
  (Transformation|SetActorLocation (Variables|Default|GetBuzzingSound) (Transformation|GetWorldLocation (Variables|Default|GetPointLight1)) false))