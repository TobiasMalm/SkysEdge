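; Corridor elevator that makes a one-way diagonal ride when anything overlaps its trigger box.
; Three chained timelines raise the rails, move the elevator along Y and up Z, then lower the rails, each offsetting from cached relative positions.
; The moving flag is never reset, so the sequence runs only once.
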(event OnComponentBeginOverlap(Box1)
  (params (OtherActor :type Actor%20Object%20Reference) (OtherComp :type Primitive%20Component%20Object%20Reference) (OtherBodyIndex :type Integer))
  (if (not (Variables|Default|GetIsElevatorMoving))
    (Variables|Default|SetIsElevatorMoving true)
    (bind _var (Timeline|ElevatorTimeline Play)
      (:Update
        (Transformation|SetRelativeLocation (Variables|Default|GetElevatorRails) (+ (Math|Vector|MakeVector 0.0 0.0 (* _var 1e+02)) (Variables|Default|GetElevatorRailsStartingPos)) false))
      (:Finished
        (Variables|Default|SetElevatorRailsStartingPos (Variables|/Script/Engine.SceneComponent|GetRelativeLocation (Variables|Default|GetElevatorRails)))
        (bind _var_2 (Timeline|Timeline_0 Play)
          (:Update
            (Transformation|SetRelativeLocation (Variables|Default|GetElevator) (+ (Math|Vector|MakeVector 0.0 (* _var_2 2003.0) (* _var_2 1997.0)) (Variables|Default|GetElevatorStartingPos)) false))
          (:Finished
            (bind _var_3 (Timeline|Timeline_1 Play)
              (:Update
                (Transformation|SetRelativeLocation (Variables|Default|GetElevatorRails) (- (Variables|Default|GetElevatorRailsStartingPos) (Math|Vector|MakeVector 0.0 0.0 (* _var_3 1e+02))) false)))))))))

(event EventBeginPlay
  (Variables|Default|SetElevatorRailsStartingPos (Variables|/Script/Engine.SceneComponent|GetRelativeLocation (Variables|Default|GetElevatorRails)))
  (Variables|Default|SetElevatorStartingPos (Variables|/Script/Engine.SceneComponent|GetRelativeLocation (Variables|Default|GetElevator))))

(fn ConstructionScript)