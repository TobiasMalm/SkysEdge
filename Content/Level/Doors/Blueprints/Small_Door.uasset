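; Small two-panel sliding door that opens on overlap with TriggerBoxOPen and closes when an overlap with TriggerBoxClose ends.
; Timelines slide LowerDoor and UpperDoor in opposite diagonal Y/Z directions from positions cached at BeginPlay, with Timeline_0 played in reverse to close.
; IsMoving prevents interrupting a motion; each finish checks IsOpen and runs the opposite motion if the state changed.
; CloseDoorTimeLine is never run.
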(event OnComponentBeginOverlap(TriggerBoxOPen)
  (params (OtherActor :type Actor%20Object%20Reference) (OtherComp :type Primitive%20Component%20Object%20Reference) (OtherBodyIndex :type Integer))
  (if (not (Variables|Default|GetIsOpen))
    (Variables|Default|SetIsOpen true)
    (if (not (Variables|Default|GetIsMoving))
      (Variables|Default|SetIsMoving true :!label _label)
      (bind _doorpos (Timeline|OpenDoorTimeLine PlayFromStart)
        (:Update
          (Transformation|SetRelativeLocation (Variables|Default|GetLowerDoor) (- (Variables|Default|GetLowerDoorInitPos) (* (Math|Vector|MakeVector 0.0 (.Z (Math|Vector|BreakVector _doorpos)) (.Z (Math|Vector|BreakVector _doorpos))) 1e+02)) false)
          (Transformation|SetRelativeLocation (Variables|Default|GetUpperDoor) (+ (Variables|Default|GetUpperDoorInitPos) (* (Math|Vector|MakeVector 0.0 (.Z (Math|Vector|BreakVector _doorpos)) (.Z (Math|Vector|BreakVector _doorpos))) 1e+02)) false))
        (:Finished
          (Variables|Default|SetIsMoving false)
          (if (not (Variables|Default|GetIsOpen))
            (Variables|Default|SetIsMoving true)
            (bind _doorpos_2 (Timeline|Timeline_0 ReverseFromEnd)
              (:Update
                (Transformation|SetRelativeLocation (Variables|Default|GetLowerDoor) (- (Variables|Default|GetLowerDoorInitPos) (* (Math|Vector|MakeVector 0.0 (.Z (Math|Vector|BreakVector _doorpos_2)) (.Z (Math|Vector|BreakVector _doorpos_2))) 1e+02)) false)
                (Transformation|SetRelativeLocation (Variables|Default|GetUpperDoor) (+ (Variables|Default|GetUpperDoorInitPos) (* (Math|Vector|MakeVector 0.0 (.Z (Math|Vector|BreakVector _doorpos_2)) (.Z (Math|Vector|BreakVector _doorpos_2))) 1e+02)) false))
              (:Finished
                (Variables|Default|SetIsMoving false)
                (if (Variables|Default|GetIsOpen)
                  (goto _label))))))))))

(event OnComponentEndOverlap(TriggerBoxClose)
  (params (OtherActor :type Actor%20Object%20Reference) (OtherComp :type Primitive%20Component%20Object%20Reference) (OtherBodyIndex :type Integer))
  (if (Variables|Default|GetIsOpen)
    (Variables|Default|SetIsOpen false)
    (if (not (Variables|Default|GetIsMoving))
      (Variables|Default|SetIsMoving true :!label _label)
      (bind _doorpos (Timeline|Timeline_0 ReverseFromEnd)
        (:Update
          (Transformation|SetRelativeLocation (Variables|Default|GetLowerDoor) (- (Variables|Default|GetLowerDoorInitPos) (* (Math|Vector|MakeVector 0.0 (.Z (Math|Vector|BreakVector _doorpos)) (.Z (Math|Vector|BreakVector _doorpos))) 1e+02)) false)
          (Transformation|SetRelativeLocation (Variables|Default|GetUpperDoor) (+ (Variables|Default|GetUpperDoorInitPos) (* (Math|Vector|MakeVector 0.0 (.Z (Math|Vector|BreakVector _doorpos)) (.Z (Math|Vector|BreakVector _doorpos))) 1e+02)) false))
        (:Finished
          (Variables|Default|SetIsMoving false)
          (if (Variables|Default|GetIsOpen)
            (Variables|Default|SetIsMoving true)
            (bind _doorpos_2 (Timeline|OpenDoorTimeLine PlayFromStart)
              (:Update
                (Transformation|SetRelativeLocation (Variables|Default|GetLowerDoor) (- (Variables|Default|GetLowerDoorInitPos) (* (Math|Vector|MakeVector 0.0 (.Z (Math|Vector|BreakVector _doorpos_2)) (.Z (Math|Vector|BreakVector _doorpos_2))) 1e+02)) false)
                (Transformation|SetRelativeLocation (Variables|Default|GetUpperDoor) (+ (Variables|Default|GetUpperDoorInitPos) (* (Math|Vector|MakeVector 0.0 (.Z (Math|Vector|BreakVector _doorpos_2)) (.Z (Math|Vector|BreakVector _doorpos_2))) 1e+02)) false))
              (:Finished
                (Variables|Default|SetIsMoving false)
                (if (not (Variables|Default|GetIsOpen))
                  (goto _label))))))))))

(event EventBeginPlay
  (Variables|Default|SetLowerDoorInitPos (Variables|/Script/Engine.SceneComponent|GetRelativeLocation (Variables|Default|GetLowerDoor)))
  (Variables|Default|SetUpperDoorInitPos (Variables|/Script/Engine.SceneComponent|GetRelativeLocation (Variables|Default|GetUpperDoor))))

(fn ConstructionScript)